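; Manager actor that drives screen vignette effects through a Niagara system held in front of the player camera.
; CallVignette queues requests with ID, duration, add-or-override and turn-off flags.
; Each tick pushes one queued request, or a default one when empty, into Niagara parameters.
; Tick also moves the actor to a set camera distance, scaling the vignette from FOV and viewport aspect to fit the view.
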(event EventTick
  (params (DeltaSeconds :type Float%20%28single-precision%29))
  (Utilities|SetPositionandLocation)
  (if (<= (Utilities|Array|Length (Variables|Default|GetVignette%20Calls%20Array)) 0)
    (CallFunction|SendVignetteCalltoNiagara (Utilities|Struct|MakeST_VignetteCall 0 0.0 false false))
    (else
      (CallFunction|SendVignetteCalltoNiagara (Utilities|Array|Get(acopy) (Variables|Default|GetVignette%20Calls%20Array)))
      (Utilities|Array|RemoveIndex (Variables|Default|GetVignette%20Calls%20Array)))))

(fn ConstructionScript)

(fn SendVignetteCalltoNiagara
  (params (Vignette%20Call :type ST%20Vignette%20Call%20Structure))
  (bind (_vignetteid _duration _adddurationinsteadofoverriding_ _turnoffvignette_) (Utilities|Struct|BreakST_VignetteCall Vignette%20Call))
  (Effects|Components|ParticleSystem|SetIntParameter (Variables|Default|GetNiagaraSystem) "VignetteIDForInteracting" _vignetteid)
  (Effects|Components|ParticleSystem|SetFloatParameter (Variables|Default|GetNiagaraSystem) "SentDuration" _duration)
  (Effects|Components|ParticleSystem|SetBoolParameter (Variables|Default|GetNiagaraSystem) "AddDurationInsteadOfOverriding?" _adddurationinsteadofoverriding_)
  (Effects|Components|ParticleSystem|SetBoolParameter (Variables|Default|GetNiagaraSystem) "KillOrder?" _turnoffvignette_))

(fn CallVignette
  (params (Vignette%20ID :type Integer) (Duration :type Float%20%28double-precision%29) (Add%20Duration%20Instead%20Of%20Overriding%20? :type Boolean) (Turn%20Off%20Vignette%20? :type Boolean))
  (Utilities|Array|Add (Variables|Default|GetVignette%20Calls%20Array) (Utilities|Struct|MakeST_VignetteCall Vignette%20ID Duration Add%20Duration%20Instead%20Of%20Overriding%20? Turn%20Off%20Vignette%20?)))