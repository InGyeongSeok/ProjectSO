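; BP_Target is a destructible target that minigun bullets wear down until it explodes.
; Each overlap with a BP_M134-Minigun-Bullet actor subtracts a small fixed amount from its health variable, named Halthe.
; Tick polls that value and, once it reaches zero or below, spawns a scaled-up P_Explosion emitter at the actor's transform and destroys the actor.
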(event EventBeginPlay)

(event Collision|EventActorBeginOverlap
  (params (OtherActor :type Actor%20Object%20Reference))
  (Utilities|Casting|CastToBP_M134-Minigun-Bullet OtherActor)
  (Variables|Default|SetHalthe (- (Variables|Default|GetHalthe) 0.01)))

(event EventTick
  (params (DeltaSeconds :type Float%20%28single-precision%29))
  (if (<= (Variables|Default|GetHalthe) 0.0)
    (Effects|SpawnEmitteratLocation "/Game/MinigunProject/VFX/P_Explosion.P_Explosion" (Transformation|GetActorLocation) (Transformation|GetActorRotation) "10.000000,10.000000,10.000000")
    (Actor|DestroyActor)))

(fn ConstructionScript)